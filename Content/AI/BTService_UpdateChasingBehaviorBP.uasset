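; Behavior tree service that feeds player-chasing state from BP_ChasingAIController into the Blackboard.
; On activation it stores the first Player actor found in the level under PlayerKey.
; Each tick it copies the controller's CanSeePlayer flag to the Blackboard.
; It writes the controller's last known player position only when that flag differs from the cached previous value, so on sight gained or lost.
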(event EventReceiveActivationAI
  (params (OwnerController :type AI%20Controller%20Object%20Reference) (ControlledPawn :type Pawn%20Object%20Reference))
  ;[1 1 1] Get a reference to the Player Actor
  (bind _outactors (Actor|GetAllActorsOfClass "/Game/ThirdPersonCPP/Blueprints/Player.Player_C"))
  (Class|BTFunctionLibrary|SetBlackboardValueasObject (Variables|Default|GetPlayerKey) (Utilities|Array|Get(acopy) _outactors)))

(event EventReceiveTickAI
  (params (OwnerController :type AI%20Controller%20Object%20Reference) (ControlledPawn :type Pawn%20Object%20Reference) (DeltaSeconds :type Float%20%28single-precision%29))
  ;[1 1 1] Update Blackboard Values
  (bind _asbp_chasing_aicontroller (Utilities|Casting|CastToBP_ChasingAIController OwnerController))
  (Class|BTFunctionLibrary|SetBlackboardValueasBool (Variables|Default|GetCanSeePlayerKey) (Variables|/Game/AI/BP_ChasingAIController.BP_ChasingAIController_C|GetbCanSeePlayer _asbp_chasing_aicontroller))
  (if (Math|Boolean|Equal(Boolean) (Variables|/Game/AI/BP_ChasingAIController.BP_ChasingAIController_C|GetbCanSeePlayer _asbp_chasing_aicontroller) (Variables|Default|GetLastCanSeePlayer))
    _
    (else
      (AI|BehaviorTree|SetBlackboardValueasVector (Variables|Default|GetLastKnownPositionKey) (Variables|/Game/AI/BP_ChasingAIController.BP_ChasingAIController_C|GetLastKnownPlayerPosition _asbp_chasing_aicontroller))))
  (Variables|Default|SetLastCanSeePlayer (Class|BTFunctionLibrary|GetBlackboardValueasBool (Variables|Default|GetCanSeePlayerKey))))